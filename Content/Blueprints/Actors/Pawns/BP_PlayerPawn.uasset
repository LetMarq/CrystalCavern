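; Player pawn that rolls a physics sphere and restarts the level when it takes any damage.
; Movement axis inputs apply torque to the sphere on the Y and X axes, scaled by Aceleration and applied as an acceleration change, so mass is ignored.
; The RestartLevel graph runs once, partially fading the camera to black and reopening the current level by name after a matching delay.
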(event Game|Damage|EventAnyDamage
  (params (Damage :type Float%20%28single-precision%29) (DamageType :type Damage%20Type%20Object%20Reference) (InstigatedBy :type Controller%20Object%20Reference) (DamageCauser :type Actor%20Object%20Reference))
  (Utilities|RestartLevel))

(event Input|AxisEvents|InputAxisMoveForwardBackwards
  (params (AxisValue :type Float%20%28single-precision%29))
  (Class|PrimitiveComponent|AddTorqueinRadians (Variables|Default|GetMeshSphere) (Math|Vector|MakeVector 0.0 (* AxisValue (Variables|Default|GetAceleration)) 0.0) "None" true))

(event Input|AxisEvents|InputAxisMoveRightLeft
  (params (AxisValue :type Float%20%28single-precision%29))
  (Class|PrimitiveComponent|AddTorqueinRadians (Variables|Default|GetMeshSphere) (Math|Vector|MakeVector (* AxisValue (Variables|Default|GetAceleration)) 0.0 0.0) "None" true))

(fn ConstructionScript)