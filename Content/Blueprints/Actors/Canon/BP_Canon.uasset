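; BP_Canon is an automatic cannon actor that repeatedly fires BP_Projectile from BeginPlay onward.
; Each cycle waits for the fire-rate delay, then spawns a scaled projectile at the spawn point's world location and rotation.
; CannonFireTimeline then animates the barrel's relative Y location, and its Cannon Fired event track loops execution back to the delay.
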(event EventBeginPlay
  (Utilities|FlowControl|Delay (Variables|CannonProperties|GetCannonFirerate) :!label _label)
  (CallFunction|SpawnProjectile)
  (bind _cannon_barrel_location (Timeline|Cannon%20Fire%20Timeline PlayFromStart)
    (:Update
      (CallFunction|MoveCannonBarrel _cannon_barrel_location))
    (:Cannon%20Fired
      (goto _label))))

(fn ConstructionScript)

(fn SpawnProjectile
  (bind _projectilespawnpoint (Variables|Default|GetProjectileSpawnPoint))
  (Game|SpawnActorfromClass "/Game/Blueprints/Actors/Projectiles/BP_Projectile.BP_Projectile_C" (Math|Transform|MakeTransform (Transformation|GetWorldLocation _projectilespawnpoint) (Transformation|GetWorldRotation _projectilespawnpoint) (Math|Conversions|ToVector(Float) (Variables|CannonProperties|GetProjectileScale))) "Undefined" 0 0))

(fn MoveCannonBarrel
  (params (CannonBarrelYLocation :type Float%20%28single-precision%29))
  (Transformation|SetRelativeLocation (Variables|Default|GetCannon) (Math|Vector|MakeVector 0.0 CannonBarrelYLocation 0.0) false false))